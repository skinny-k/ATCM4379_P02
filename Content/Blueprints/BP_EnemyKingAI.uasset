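; Gold-skinned enemy king character for a VR giant game, which flees or chases and bayonet-stabs the player depending on IsCoward.
; Pawn sensing triggers AI moves; the RethinkLifeChoices hook is empty and the random coward roll is unwired.
; The giant can grab the king, suspending movement, or eat him via the mouth sensor, changing giant health.
; Eating or hard impacts cause ragdoll and blood explosion, then announce the king's death and destroy him.
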(event OnSeePawn(PawnSensing)
  (params (Pawn :type Pawn%20Object%20Reference))
  (Variables|Default|SetSaw%20Player true)
  (Variables|Default|SetSees%20Player? true)
  (if (Variables|Default|GetisCoward?)
    (CallFunction|FleePlayer)
    (else
      (CallFunction|FollowPlayer)
      (Utilities|FlowControl|DoOnce false
        (:Completed
          (Variables|Default|SetCanAttack? true))))))

(event OnComponentBeginOverlap(CapsuleComponent)
  (params (OverlappedComponent :type Primitive%20Component%20Object%20Reference) (OtherActor :type Actor%20Object%20Reference) (OtherComp :type Primitive%20Component%20Object%20Reference) (OtherBodyIndex :type Integer) (bFromSweep :type Boolean) (SweepResult :type Hit%20Result%20Structure%20%28by%20ref%29))
  (if (== OtherComp (Variables|Default|GetGiantMouth))
    (CallFunction|EatMe)))

(event OnComponentActivated(BloodExplosion)
  (params (Component :type Actor%20Component%20Object%20Reference) (bReset :type Boolean))
  (Audio|PlaySoundatLocation 0 (Transformation|GetActorLocation) "0, 0, 0" 1.0 1.0 0.0 0 0 0 0)
  (Utilities|FlowControl|Delay 3.0)
  (Default|CallKingDies)
  (Actor|DestroyActor))

(event OnDropped(GrabComponent)
  (Physics|SetEnableGravity (Variables|Collision|GetCapsuleComponent) true)
  (Variables|Default|SetisGrabbed? false)
  (Pawn|Components|CharacterMovement|SetMovementMode (Variables|Character|GetCharacterMovement) "MOVE_Walking" 0))

(event OnGrabbed(GrabComponent)
  (Physics|SetEnableGravity (Variables|Collision|GetCapsuleComponent) false)
  (Variables|Default|SetisGrabbed? true)
  (Pawn|Components|CharacterMovement|DisableMovement (Variables|Character|GetCharacterMovement))
  (Animation|PlayAnimMontage "/Game/Animations/Villager/Bayonet_Stab_Montage.Bayonet_Stab_Montage" 1.0 "None"))

(event OnComponentHit(CapsuleComponent)
  (params (HitComponent :type Primitive%20Component%20Object%20Reference) (OtherActor :type Actor%20Object%20Reference) (OtherComp :type Primitive%20Component%20Object%20Reference) (NormalImpulse :type Vector :default "0, 0, 0") (Hit :type Hit%20Result%20Structure%20%28by%20ref%29))
  (if (>= (Math|Vector|VectorLength NormalImpulse) (Variables|Default|GetMaxForce))
    (CallFunction|GoRagdoll)
    (Components|Activation|Activate (Variables|Default|GetBloodExplosion) false)))

(event Custom|FollowPlayer
  ;[1 1 1] Follow and Attack Player
  (if (Variables|Default|GetSees%20Player?)
    (AI|AIMoveTo self "0, 0, 0" (Game|Player|GetPlayerPawn 0) 2e+02 false
      (:OnSuccess
        (if (Variables|Default|GetCanAttack?)
          (Variables|Default|SetCanAttack? false)
          (bind _returnvalue (Animation|PlayAnimMontage "/Game/Animations/Villager/Bayonet_Stab_Montage.Bayonet_Stab_Montage" 1.0 "None"))
          (Default|EventAnyDamage (Variables|/Game/VRTemplate/Blueprints/VRPawn_Giant.VRPawn_Giant_C|GetBP_Health (Variables|Components|GetVRPawn%20Giant)) -2.0)
          (Utilities|FlowControl|Delay (- _returnvalue 1.0))
          (CallFunction|RethinkLifeChoices)
          (Variables|Default|SetCanAttack? true))))))

(event Custom|FleePlayer
  (bind _returnvalue (Game|Player|GetPlayerPawn 0))
  (bind _returnvalue_2 (Transformation|GetActorLocation))
  (bind _returnvalue_3 (Math|Conversions|ToVector(Float) -5e+02))
  (bind _returnvalue_4 (Transformation|GetActorLocation _returnvalue))
  (bind _returnvalue_5 (Math|Rotator|FindLookatRotation _returnvalue_2 _returnvalue_4))
  (bind _returnvalue_6 (Math|Vector|GetForwardVector _returnvalue_5))
  (bind _returnvalue_7 (* _returnvalue_6 _returnvalue_3))
  (bind _returnvalue_8 (+ _returnvalue_2 _returnvalue_7))
  (bind _returnvalue_9 (+ _returnvalue_8 "200.000000,200.000000,0.000000"))
  (bind (_x _y) (Math|Vector|BreakVector _returnvalue_9))
  ;[1 1 1] Flee From Player
  (AI|AIMoveTo self (Math|Vector|MakeVector _x _y (.Z (Math|Vector|BreakVector _returnvalue_2))) 0 5.0 false
    (:OnSuccess
      (CallFunction|RethinkLifeChoices))))

(event Custom|RethinkLifeChoices)

(event Custom|GoRagdoll
  (Physics|SetSimulatePhysics (Variables|Character|GetMesh) true)
  (Collision|SetCollisionProfileName (Variables|Character|GetMesh) "Ragdoll" true :!class /Script/Engine.PrimitiveComponent))

(event Custom|Eat%20Me
  (Rendering|SetVisibility (Variables|Character|GetMesh) false false)
  (Components|Activation|Activate (Variables|Default|GetBloodExplosion) false)
  (CallFunction|GoRagdoll)
  (Default|EventAnyDamage (Variables|/Game/VRTemplate/Blueprints/VRPawn_Giant.VRPawn_Giant_C|GetBP_Health (Variables|Components|GetVRPawn%20Giant)) 3e+01))

(event EventBeginPlay
  (CallFunction|RethinkLifeChoices)
  (bind _returnvalue (Actor|GetActorOfClass "/Game/VRTemplate/Blueprints/VRPawn_Giant.VRPawn_Giant_C"))
  (Variables|Components|SetVRPawn%20Giant _returnvalue)
  (Variables|Default|SetGiantMouth (Variables|/Game/VRTemplate/Blueprints/VRPawn_Giant.VRPawn_Giant_C|GetMouthSensor _returnvalue)))

(event Collision|EventActorBeginOverlap
  (params (OtherActor :type Actor%20Object%20Reference)))

(event EventTick
  (params (DeltaSeconds :type Float%20%28single-precision%29))
  (if (not (Variables|Default|GetisGrabbed?))
    (if (Variables|Default|GetSaw%20Player)
      (if (Variables|Default|GetisCoward?)
        (CallFunction|FleePlayer)
        (Utilities|FlowControl|Delay 2e+01)
        (CallFunction|RethinkLifeChoices)
        (elif (not (Variables|Default|GetSees%20Player?))
          (Components|Movement|StopMovementImmediately (Variables|Character|GetCharacterMovement))
          (CallFunction|RethinkLifeChoices))))))

(fn ConstructionScript
  (Rendering|Material|SetMaterial (Variables|Character|GetMesh) 0 "/Game/Materials/M_Gold.M_Gold"))