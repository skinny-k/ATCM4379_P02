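; FlyingRock is an unfinished Blueprint for a rock meant to be thrown at a target, with no active gameplay logic.
; Its disconnected graph chains contain an AI move-to call and an impulse on the Rock component, scaled by ImpulseValue.
; CalculateThrowVelocity supplies that impulse via a suggested custom-arc projectile velocity from the owner's location.
; The arc's end offset is multiplied by zero, so it ends where it starts.
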(event EventBeginPlay)

(event Collision|EventActorBeginOverlap
  (params (OtherActor :type Actor%20Object%20Reference)))

(event EventTick
  (params (DeltaSeconds :type Float%20%28single-precision%29)))

(fn ConstructionScript)

(fn CalculateThrowVelocity
  (params (Rotation :type Rotator))
  (bind _returnvalue (Components|GetOwner))
  (bind _returnvalue_2 (Transformation|GetActorLocation _returnvalue))
  (bind _outlaunchvelocity (Game|SuggestProjectileVelocityCustomArc _returnvalue_2 (+ _returnvalue_2 (* (Math|Rotator|GetRotationXVector Rotation) "")) 0.0 0.5))
  (return _outlaunchvelocity))