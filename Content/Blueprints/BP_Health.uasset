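; BP_Health is a health Blueprint that tracks current health and initializes it on BeginPlay.
; AnyDamage adds the incoming Damage to current health, so positive values raise it, clamps it between zero and MaxHealth, then calls UpdateHealth with both values.
; Tick checks for depleted health, but the branch is empty, and killing the parent exists only as a comment.
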(event Custom|EventAnyDamage
  (params (Damage :type Float%20%28double-precision%29))
  (bind _maxhealth (Variables|Default|GetmaxHealth))
  (Variables|Default|SetcurrentHealth (Math|Float|Clamp(Float) (+ (Variables|Default|GetcurrentHealth) Damage) 0.0 _maxhealth))
  (Default|CallUpdateHealth (Variables|Default|GetcurrentHealth) _maxhealth))

(event EventBeginPlay
  (Variables|Default|SetcurrentHealth 1e+02))

(event EventTick
  (params (DeltaSeconds :type Float%20%28single-precision%29))
  (if (<= (Variables|Default|GetcurrentHealth) 0.0) ; if health under or equal to 0, kill parent
    _))