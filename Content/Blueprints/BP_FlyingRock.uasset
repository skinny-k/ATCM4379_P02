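; BP_FlyingRock is a rock actor that launches itself by physics impulse, meant to be thrown at the VR giant player.
; BeginPlay stores the player pawn as Target if it is a VRPawn_Giant.
; ThrowRock applies a custom-arc projectile velocity, scaled by ImpulseValue, as an impulse on Rock.
; The arc's endpoint offsets the rock's position along X by the target's scaled world X, rather than using the target's position directly.
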(event Custom|ThrowRock
  (Utilities|IsValid 0
    (:Is%20Valid
      (Utilities|String|LogString "tried throw rock")
      (bind _launch_velocity (CallFunction|CalculateThrowVelocity (Transformation|GetActorLocation (stale EventBeginPlay _output_get))))
      (Physics|AddImpulse (Variables|Default|GetRock) (* _launch_velocity (Variables|Default|GetImpulseValue)) "None" false))))

(event EventBeginPlay
  (bind _returnvalue (Game|Player|GetPlayerPawn 0))
  (Utilities|String|LogString "tried throw rock")
  (Utilities|Casting|CastToVRPawn_Giant _returnvalue)
  (bind _output_get (Variables|Default|SetTarget _returnvalue)))

(event EventTick
  (params (DeltaSeconds :type Float%20%28single-precision%29)))

(fn ConstructionScript)

(fn CalculateThrowVelocity
  (params (Location :type Vector))
  (bind _returnvalue (Transformation|GetActorLocation))
  (bind (_outlaunchvelocity _returnvalue_2) (Game|SuggestProjectileVelocityCustomArc _returnvalue (+ _returnvalue (* Location "750.000000,0.000000,0.000000")) 0.0 0.5))
  (return _outlaunchvelocity _returnvalue_2))