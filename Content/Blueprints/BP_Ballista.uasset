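; BP_Ballista is a turret that shoots oversized BP_FlyingRock projectiles at the VR giant player and is destroyed when hit by a rock or the giant.
; Tick accumulates a timer, firing once it matures with the player in range, or every frame while Enabled is false.
; Before each shot it turns toward the player at its own height with a yaw offset, then launches a player-damaging rock by impulse along its scaled, negated right vector.
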(event Custom|Fire
  (bind _returnvalue (Game|SpawnActorfromClass "/Game/Blueprints/BP_FlyingRock.BP_FlyingRock_C" (Transformation|GetWorldTransform (Variables|Default|GetProjectile%20Origin)) "AdjustIfPossibleButAlwaysSpawn" 0 0))
  (Variables|/Game/Blueprints/BP_FlyingRock.BP_FlyingRock_C|SetHurts%20Player _returnvalue true)
  (Transformation|SetActorScale3D _returnvalue "50.000000,50.000000,50.000000")
  (Physics|AddImpulse (Variables|/Game/Blueprints/BP_FlyingRock.BP_FlyingRock_C|GetRock _returnvalue) (* (* (Variables|Default|GetLaunch%20Force) (Transformation|GetActorRightVector)) "-1.000000,-1.000000,-2.000000") "None" false)
  (Variables|Default|SetTimer 0.0))

(event Custom|TargetPlayer
  (bind _returnvalue (Transformation|GetActorLocation))
  (bind _player (Variables|Default|GetPlayer))
  (bind _returnvalue_2 (Transformation|GetActorLocation _player))
  (bind (_x _y) (Math|Vector|BreakVector _returnvalue_2))
  (Transformation|SetActorRotation (Math|Rotator|CombineRotators "0.000000,92.500000,0.000000" (Math|Rotator|FindLookatRotation _returnvalue (Math|Vector|MakeVector _x _y (.Z (Math|Vector|BreakVector _returnvalue)))))))

(event EventBeginPlay
  (Variables|Default|SetTimer 0.0)
  (bind _returnvalue (Actor|GetActorOfClass "/Game/VRTemplate/Blueprints/VRPawn_Giant.VRPawn_Giant_C"))
  (Variables|Default|SetPlayer _returnvalue))

(event Collision|EventHit
  (params (MyComp :type Primitive%20Component%20Object%20Reference) (Other :type Actor%20Object%20Reference) (OtherComp :type Primitive%20Component%20Object%20Reference) (bSelfMoved :type Boolean) (HitLocation :type Vector :default "0, 0, 0") (HitNormal :type Vector :default "0, 0, 0") (NormalImpulse :type Vector :default "0, 0, 0") (Hit :type Hit%20Result%20Structure%20%28by%20ref%29))
  (Utilities|Casting|CastToBP_FlyingRock Other
    (:then
      _)
    (:CastFailed
      (Utilities|Casting|CastToVRPawn_Giant Other)))
  (Actor|DestroyActor))

(event EventTick
  (params (DeltaSeconds :type Float%20%28single-precision%29))
  (if (and (Math|Boolean|NANDBoolean (<= (Math|Vector|Distance(Vector) (Transformation|GetActorLocation) (Transformation|GetActorLocation (Variables|Default|GetPlayer))) (Variables|Default|GetRange)) (>= (Variables|Default|GetTimer) (Variables|Default|GetMax%20Shot%20Timer))) (Variables|Default|GetEnabled))
    (Variables|Default|SetTimer (+ (Variables|Default|GetTimer) DeltaSeconds))
    (else
      (CallFunction|TargetPlayer)
      (CallFunction|Fire))))

(fn ConstructionScript)